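; Procedural 2D level generator that builds a random connected path of terrain tiles on Begin Play and clears its map when Space is pressed.
; A random walk starts at the grid center and repeatedly exits through a random open side into a vacant neighbor.
; Shuffled type and rotation pairs are tested until one connects back to the previous tile.
; Tile data lives in a flattened array and renders as Paper2D grouped sprite instances with backgrounds.
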(event `self.ReceiveBeginPlay`
  (bind _tilemap (`self.tileMap`))
  (bind _mapsize (`self.mapSize`))
  (bind _mapsize_2 (`self.mapSize`))
  (bind _returnvalue (+ (* _mapsize 2) 1))
  ;[1 1 1] can't recieve input without these nodes
  (`self.EnableInput` (`GameplayStatics.GetPlayerController` 0))
  (if (not (`KismetMathLibrary.Conv_IntToBool` (mod _mapsize 2))) :!label _label
    (`/Engine/EditorBlueprintResources/StandardMacros.IncrementInt` _mapsize
      (:`  `
        _)))
  (set `self.width` _returnvalue)
  (set `self.height` _returnvalue)
  (`KismetArrayLibrary.Array_Resize` (`self.tileMap`) (* (`self.height`) (`self.width`)))
  (for (_ _array_index) _tilemap
    (`KismetArrayLibrary.Array_Set` _tilemap _array_index (make `/Game/Blueprints/Structs/TileInformation` -1)))
  (bind _output_get (set `self.currX` _mapsize_2))
  (set `self.prevX` _output_get)
  (bind _output_get_2 (set `self.currZ` _mapsize_2))
  (set `self.prevZ` _output_get_2)
  ;[1 1 1] create and place the middle tile before starting to loop
  (`self.PickAndSetRandomTileInformation` (`self.currX`) (`self.currZ`))
  (`self.PlaceTile`)
  (for _ (range (+ (- (`self.mapSize`) 2) 1))
    ;[1 1 1] the basic loop for populating the rest of the tile map
    (bind _dir (`self.PickAndSetDirection` (`self.currX`) (`self.currZ`)))
    (`self.MatchAdjacentOpenings` _dir)
    (`self.PlaceTile`)
    (set `self.prevX` (`self.currX`))
    (set `self.prevZ` (`self.currZ`))))

(event `Key|SpaceBar`
  (params (Key :type "Key Structure" :default "AnyKey"))
  (:`Pressed`
    (`PaperGroupedSpriteComponent.ClearInstances` (`self.BackgroundPaperGroupedSprite`))
    (`PaperGroupedSpriteComponent.ClearInstances` (`self.CornerPaperGroupedSprite`))
    (`PaperGroupedSpriteComponent.ClearInstances` (`self.DeadEndPaperGroupedSprite`))
    (`PaperGroupedSpriteComponent.ClearInstances` (`self.FourWayPaperGroupedSprite`))
    (`PaperGroupedSpriteComponent.ClearInstances` (`self.StraightPaperGroupedSprite`))
    (`PaperGroupedSpriteComponent.ClearInstances` (`self.ThreeWayPaperGroupedSprite`))
    (`KismetArrayLibrary.Array_Clear` (`self.tileMap`))
    (goto _label)))

(fn `FindAndSetOpenings`
  (params (x :type Integer) (z :type Integer))
  (locals (availableOpenings :type Integer) (xCheck :type Integer) (zCheck :type Integer) (NewLocalVar_0 :type Integer))
  (bind _xcheck (`local.xCheck`))
  (bind _zcheck (`local.zCheck`))
  (bind _zcheck_2 (`local.zCheck`))
  (bind _xcheck_2 (`local.xCheck`))
  (bind _xcheck_3 (`local.xCheck`))
  (bind _zcheck_3 (`local.zCheck`))
  (bind _xcheck_4 (`local.xCheck`))
  (bind _zcheck_4 (`local.zCheck`))
  (bind _xcheck_5 (`local.xCheck`))
  (bind _zcheck_5 (`local.zCheck`))
  (bind _xcheck_6 (`local.xCheck`))
  (bind _zcheck_6 (`local.zCheck`))
  (bind _xcheck_7 (`local.xCheck`))
  (bind _zcheck_7 (`local.zCheck`))
  (bind _xcheck_8 (`local.xCheck`))
  (bind _zcheck_8 (`local.zCheck`))
  (bind _xcheck_9 (`local.xCheck`))
  (bind _zcheck_9 (`local.zCheck`))
  (bind _xcheck_10 (`local.xCheck`))
  (bind _zcheck_10 (`local.zCheck`))
  (set `local.xCheck` x)
  (set `local.zCheck` z)
  (bind _element (`self.GetTileInfo` x z))
  (`self.Which Tile` (break `/Game/Blueprints/Structs/TileInformation` _element)
    (:`Vacant`
      _)
    (:`Four Way`
      ;[1 1 1] each tile type has a unique layout
      (bind _isvacant (`self.SetTopVacancy` _xcheck_4 _zcheck_4))
      (if _isvacant
        (`/Engine/EditorBlueprintResources/StandardMacros.IncrementInt` (`local.availableOpenings`)
          (:`  `
            _)))
      (bind _isvacant_2 (`self.SetBottomVacancy` _xcheck_4 _zcheck_4))
      (if _isvacant_2
        (`/Engine/EditorBlueprintResources/StandardMacros.IncrementInt` (`local.availableOpenings`)
          (:`  `
            _)))
      (bind _isvacant_3 (`self.SetLeftVacancy` _xcheck_4 _zcheck_4))
      (if _isvacant_3
        (`/Engine/EditorBlueprintResources/StandardMacros.IncrementInt` (`local.availableOpenings`)
          (:`  `
            _)))
      (bind _isvacant_4 (`self.SetRightVacancy` _xcheck_4 _zcheck_4))
      (if _isvacant_4
        (`/Engine/EditorBlueprintResources/StandardMacros.IncrementInt` (`local.availableOpenings`)
          (:`  `
            _)))
      ;[1 1 1] save the available openings total before we leave
      (bind _element_2 (`self.GetTileInfo` _xcheck_10 _zcheck_10 :!label _label))
      (`self.SetTileInfo` (make `/Game/Blueprints/Structs/TileInformation` (break `/Game/Blueprints/Structs/TileInformation` _element_2) (`.Rotation_5_ADDC5B57482A9A9A5491C3B6ED31BCB7` (break `/Game/Blueprints/Structs/TileInformation` _element_2)) (`local.availableOpenings`) (`.Left_10_DB7199D24824B389FF47D582AEDECBFF` (break `/Game/Blueprints/Structs/TileInformation` _element_2)) (`.Right_14_58CFD1D541F441DB794B599FE93CD335` (break `/Game/Blueprints/Structs/TileInformation` _element_2)) (`.Top_15_FF8EB3A44EBFBDEC54CE4783EB41D170` (break `/Game/Blueprints/Structs/TileInformation` _element_2)) (`.Down_16_1ABB1D3F4A6AF141A8692C870330AC01` (break `/Game/Blueprints/Structs/TileInformation` _element_2))) _xcheck_10 _zcheck_10))
    (:`Straight`
      (`self.What Degree` (`.Rotation_5_ADDC5B57482A9A9A5491C3B6ED31BCB7` (break `/Game/Blueprints/Structs/TileInformation` _element))
        (:`0`
          _)
        (:`90`
          (bind _isvacant_5 (`self.SetTopVacancy` _xcheck_5 _zcheck_5 :!label _label_2))
          (if _isvacant_5
            (`/Engine/EditorBlueprintResources/StandardMacros.IncrementInt` (`local.availableOpenings`)
              (:`  `
                _)))
          (bind _isvacant_6 (`self.SetBottomVacancy` _xcheck_5 _zcheck_5))
          (if _isvacant_6
            (`/Engine/EditorBlueprintResources/StandardMacros.IncrementInt` (`local.availableOpenings`)
              (:`  `
                (goto _label)))
            (else
              (goto _label))))
        (:`180`
          _)
        (:`270`
          (goto _label_2)))
      (bind _isvacant_7 (`self.SetRightVacancy` _xcheck_5 _zcheck_5))
      (if _isvacant_7
        (`/Engine/EditorBlueprintResources/StandardMacros.IncrementInt` (`local.availableOpenings`)
          (:`  `
            _)))
      (bind _isvacant_8 (`self.SetLeftVacancy` _xcheck_5 _zcheck_5))
      (if _isvacant_8
        (`/Engine/EditorBlueprintResources/StandardMacros.IncrementInt` (`local.availableOpenings`)
          (:`  `
            (goto _label)))
        (else
          (goto _label))))
    (:`Three Way`
      (`self.What Degree` (`.Rotation_5_ADDC5B57482A9A9A5491C3B6ED31BCB7` (break `/Game/Blueprints/Structs/TileInformation` _element))
        (:`0`
          (bind _isvacant_9 (`self.SetLeftVacancy` _xcheck_6 _zcheck_6))
          (if _isvacant_9
            (`/Engine/EditorBlueprintResources/StandardMacros.IncrementInt` (`local.availableOpenings`)
              (:`  `
                _)))
          (bind _isvacant_10 (`self.SetRightVacancy` _xcheck_6 _zcheck_6))
          (if _isvacant_10
            (`/Engine/EditorBlueprintResources/StandardMacros.IncrementInt` (`local.availableOpenings`)
              (:`  `
                _)))
          (bind _isvacant_11 (`self.SetTopVacancy` _xcheck_6 _zcheck_6))
          (if _isvacant_11
            (`/Engine/EditorBlueprintResources/StandardMacros.IncrementInt` (`local.availableOpenings`)
              (:`  `
                (goto _label)))
            (else
              (goto _label))))
        (:`90`
          (bind _isvacant_12 (`self.SetTopVacancy` _xcheck_7 _zcheck_7))
          (if _isvacant_12
            (`/Engine/EditorBlueprintResources/StandardMacros.IncrementInt` (`local.availableOpenings`)
              (:`  `
                _)))
          (bind _isvacant_13 (`self.SetRightVacancy` _xcheck_7 _zcheck_7))
          (if _isvacant_13
            (`/Engine/EditorBlueprintResources/StandardMacros.IncrementInt` (`local.availableOpenings`)
              (:`  `
                _)))
          (bind _isvacant_14 (`self.SetBottomVacancy` _xcheck_7 _zcheck_7))
          (if _isvacant_14
            (`/Engine/EditorBlueprintResources/StandardMacros.IncrementInt` (`local.availableOpenings`)
              (:`  `
                (goto _label)))
            (else
              (goto _label))))
        (:`180`
          (bind _isvacant_15 (`self.SetLeftVacancy` _xcheck_8 _zcheck_8))
          (if _isvacant_15
            (`/Engine/EditorBlueprintResources/StandardMacros.IncrementInt` (`local.availableOpenings`)
              (:`  `
                _)))
          (bind _isvacant_16 (`self.SetRightVacancy` _xcheck_8 _zcheck_8))
          (if _isvacant_16
            (`/Engine/EditorBlueprintResources/StandardMacros.IncrementInt` (`local.availableOpenings`)
              (:`  `
                _)))
          (bind _isvacant_17 (`self.SetBottomVacancy` _xcheck_8 _zcheck_8))
          (if _isvacant_17
            (`/Engine/EditorBlueprintResources/StandardMacros.IncrementInt` (`local.availableOpenings`)
              (:`  `
                (goto _label)))
            (else
              (goto _label))))
        (:`270`
          (bind _isvacant_18 (`self.SetTopVacancy` _xcheck_9 _zcheck_9))
          (if _isvacant_18
            (`/Engine/EditorBlueprintResources/StandardMacros.IncrementInt` (`local.availableOpenings`)
              (:`  `
                _)))
          (bind _isvacant_19 (`self.SetBottomVacancy` _xcheck_9 _zcheck_9))
          (if _isvacant_19
            (`/Engine/EditorBlueprintResources/StandardMacros.IncrementInt` (`local.availableOpenings`)
              (:`  `
                _)))
          (bind _isvacant_20 (`self.SetLeftVacancy` _xcheck_9 _zcheck_9))
          (if _isvacant_20
            (`/Engine/EditorBlueprintResources/StandardMacros.IncrementInt` (`local.availableOpenings`)
              (:`  `
                (goto _label)))
            (else
              (goto _label))))))
    (:`Corner`
      (`self.What Degree` (`.Rotation_5_ADDC5B57482A9A9A5491C3B6ED31BCB7` (break `/Game/Blueprints/Structs/TileInformation` _element))
        (:`0`
          (bind _isvacant_21 (`self.SetTopVacancy` _xcheck _zcheck))
          (if _isvacant_21
            (`/Engine/EditorBlueprintResources/StandardMacros.IncrementInt` (`local.availableOpenings`)
              (:`  `
                _)))
          (bind _isvacant_22 (`self.SetLeftVacancy` _xcheck _zcheck))
          (if _isvacant_22
            (`/Engine/EditorBlueprintResources/StandardMacros.IncrementInt` (`local.availableOpenings`)
              (:`  `
                (goto _label)))
            (else
              (goto _label))))
        (:`90`
          (bind _isvacant_23 (`self.SetTopVacancy` _xcheck _zcheck))
          (if _isvacant_23
            (`/Engine/EditorBlueprintResources/StandardMacros.IncrementInt` (`local.availableOpenings`)
              (:`  `
                _)))
          (bind _isvacant_24 (`self.SetRightVacancy` _xcheck _zcheck))
          (if _isvacant_24
            (`/Engine/EditorBlueprintResources/StandardMacros.IncrementInt` (`local.availableOpenings`)
              (:`  `
                (goto _label)))
            (else
              (goto _label))))
        (:`180`
          (bind _isvacant_25 (`self.SetRightVacancy` _xcheck_2 _zcheck_2))
          (if _isvacant_25
            (`/Engine/EditorBlueprintResources/StandardMacros.IncrementInt` (`local.availableOpenings`)
              (:`  `
                _)))
          (bind _isvacant_26 (`self.SetBottomVacancy` _xcheck_2 _zcheck_2))
          (if _isvacant_26
            (`/Engine/EditorBlueprintResources/StandardMacros.IncrementInt` (`local.availableOpenings`)
              (:`  `
                (goto _label)))
            (else
              (goto _label))))
        (:`270`
          (bind _isvacant_27 (`self.SetLeftVacancy` _xcheck_2 _zcheck_2))
          (if _isvacant_27
            (`/Engine/EditorBlueprintResources/StandardMacros.IncrementInt` (`local.availableOpenings`)
              (:`  `
                _)))
          (bind _isvacant_28 (`self.SetBottomVacancy` _xcheck_2 _zcheck_2))
          (if _isvacant_28
            (`/Engine/EditorBlueprintResources/StandardMacros.IncrementInt` (`local.availableOpenings`)
              (:`  `
                (goto _label)))
            (else
              (goto _label))))))
    (:`Dead End`
      (`self.What Degree` (`.Rotation_5_ADDC5B57482A9A9A5491C3B6ED31BCB7` (break `/Game/Blueprints/Structs/TileInformation` _element))
        (:`0`
          (bind _isvacant_29 (`self.SetLeftVacancy` _xcheck_3 _zcheck_3))
          (if _isvacant_29
            (`/Engine/EditorBlueprintResources/StandardMacros.IncrementInt` (`local.availableOpenings`)
              (:`  `
                (goto _label)))
            (else
              (goto _label))))
        (:`90`
          (bind _isvacant_30 (`self.SetTopVacancy` _xcheck_3 _zcheck_3))
          (if _isvacant_30
            (`/Engine/EditorBlueprintResources/StandardMacros.IncrementInt` (`local.availableOpenings`)
              (:`  `
                (goto _label)))
            (else
              (goto _label))))
        (:`180`
          (bind _isvacant_31 (`self.SetRightVacancy` _xcheck_3 _zcheck_3))
          (if _isvacant_31
            (`/Engine/EditorBlueprintResources/StandardMacros.IncrementInt` (`local.availableOpenings`)
              (:`  `
                (goto _label)))
            (else
              (goto _label))))
        (:`270`
          (bind _isvacant_32 (`self.SetBottomVacancy` _xcheck_3 _zcheck_3))
          (if _isvacant_32
            (`/Engine/EditorBlueprintResources/StandardMacros.IncrementInt` (`local.availableOpenings`)
              (:`  `
                (goto _label)))
            (else
              (goto _label)))))))
  (return))

(fn `GetTileInfo`
  (params (xGet :type Integer) (zGet :type Integer))
  (returns (element :type "/Game/Blueprints/Structs/TileInformation Structure"))
  (return (`KismetArrayLibrary.Array_Get` (`self.tileMap`) (+ xGet (* zGet (`self.width`))))))

(fn `MatchAdjacentOpenings`
  (params (Direction :type Integer))
  (locals (fromDirection :type Integer))
  (bind _currx (`self.currX`))
  (bind _currz (`self.currZ`))
  (set `local.fromDirection` Direction)
  ;[1 1 1] create and shuffle arrays for tile type and rotations
  (bind _randomints (`self.Shuffle` 4))
  (bind _randomints_2 (`self.Shuffle` 4))
  ;[1 1 1] iterate through until a working combination is found
  (for _array_element _randomints
    (for _array_element_2 _randomints_2
      (`self.SetTileInfo` (make `/Game/Blueprints/Structs/TileInformation` _array_element _array_element_2) _currx _currz)
      (set `self.dontCheckDirections` true)
      (`self.FindAndSetOpenings` _currx _currz)
      (bind _element (`self.GetTileInfo` _currx _currz))
      (`self.Match From Direction` (`local.fromDirection`) (`.Left_10_DB7199D24824B389FF47D582AEDECBFF` (break `/Game/Blueprints/Structs/TileInformation` _element)) (`.Right_14_58CFD1D541F441DB794B599FE93CD335` (break `/Game/Blueprints/Structs/TileInformation` _element)) (`.Top_15_FF8EB3A44EBFBDEC54CE4783EB41D170` (break `/Game/Blueprints/Structs/TileInformation` _element)) (`.Down_16_1ABB1D3F4A6AF141A8692C870330AC01` (break `/Game/Blueprints/Structs/TileInformation` _element))
        (:`matched`
          ;[1 1 1] check and set our openings once we found the right tile and rotation
          (set `self.dontCheckDirections` false :!label _label)
          (`self.FindAndSetOpenings` (`self.currX`) (`self.currZ`))
          (return)))))
  ;[1 0.08689 0.9273] for debug use
  (`KismetSystemLibrary.PrintString` "Matching Failure!")
  (goto _label))

(fn `PickAndSetDirection`
  (params (x :type Integer) (z :type Integer))
  (returns (Dir :type Integer))
  (locals (xCheck :type Integer :default 0) (zCheck :type Integer :default 0))
  (bind _output_get (set `local.xCheck` x))
  (bind _output_get_2 (set `local.zCheck` z))
  (bind _element (`self.GetTileInfo` _output_get _output_get_2))
  ;[1 1 1] so long we aren't in a vacant tile and have available openings, we can pick where we want to go
  (if (> (`.Openings_7_F7EF8F88495907CF6207A0B58024D475` (break `/Game/Blueprints/Structs/TileInformation` _element)) 0)
    (`self.Which Tile` (break `/Game/Blueprints/Structs/TileInformation` _element)
      (:`Vacant`
        ;[1 0.2486 0.8262] for debug use
        (`KismetSystemLibrary.PrintString` "Vacant tile!"))
      (:`Four Way`
        (bind (_vacantx _vacantz _direction) (`self.PickRandomVacancy` (`local.xCheck`) (`local.zCheck`) :!label _label))
        (set `self.currX` _vacantx)
        (set `self.currZ` _vacantz))
      (:`Straight`
        (goto _label))
      (:`Three Way`
        (goto _label))
      (:`Corner`
        (goto _label))
      (:`Dead End`
        (goto _label)))
    (else
      (`KismetSystemLibrary.PrintString` "No openings available!")))
  (return _direction))

(fn `PickAndSetRandomTileInformation`
  (params (x :type Integer) (z :type Integer))
  (`self.SetTileInfo` (make `/Game/Blueprints/Structs/TileInformation` (`KismetMathLibrary.RandomIntegerInRange` 0 3) (`KismetMathLibrary.RandomIntegerInRange` 0 3)) x z)
  ;[1 1 1] figure out and set the rest of the information
  (`self.FindAndSetOpenings` x z)
  (return))

(fn `PickRandomVacancy`
  (params (SourceX :type Integer) (sourceZ :type Integer))
  (returns (vacantX :type Integer) (vacantZ :type Integer) (direction :type Integer))
  (locals (xCheck :type Integer) (zCheck :type Integer))
  (set `local.xCheck` SourceX)
  (set `local.zCheck` sourceZ)
  ;[1 1 1] iterate through all possible directions until one that works is found, then close that direction
  (bind _randomints (`self.Shuffle` 4))
  (for _array_element _randomints
    (`self.Close Opening If Able` _array_element (`local.xCheck`) (`local.zCheck`)
      (:`leftClosed`
        ;[1 1 1] move our x or z variable to the vacant position
        (`/Engine/EditorBlueprintResources/StandardMacros.DecrementInt` (`local.xCheck`)
          (:`  `
            _)))
      (:`rightClosed`
        (`/Engine/EditorBlueprintResources/StandardMacros.IncrementInt` (`local.xCheck`)
          (:`  `
            _)))
      (:`topClosed`
        (`/Engine/EditorBlueprintResources/StandardMacros.IncrementInt` (`local.zCheck`)
          (:`  `
            _)))
      (:`downClosed`
        (`/Engine/EditorBlueprintResources/StandardMacros.DecrementInt` (`local.zCheck`)
          (:`  `
            _))))
    (return (`local.xCheck`) (`local.zCheck`) _array_element))
  ;[1 0.1101 0.8762] for debug use
  (`KismetSystemLibrary.PrintString` "Unable to close opening!")
  (return (`local.xCheck`) (`local.zCheck`) _array_element))

(fn `PlaceTile`
  (bind _currx (`self.currX`))
  (bind _currz (`self.currZ`))
  (bind _tilesize (`self.tileSize`))
  (bind _element (`self.GetTileInfo` _currx _currz))
  ;[1 1 1] determine what tile we are working with, then create an instance of the tile as well as a background
  (`self.Which Tile` (break `/Game/Blueprints/Structs/TileInformation` _element)
    (:`Vacant`
      _)
    (:`Four Way`
      (bind _returnvalue (`KismetMathLibrary.MakeTransform` (`KismetMathLibrary.MakeVector` (`KismetMathLibrary.Conv_IntToDouble` (* _currx _tilesize)) 0.0 (`KismetMathLibrary.Conv_IntToDouble` (* _currz _tilesize))) (`KismetMathLibrary.MakeRotator` 0.0 (* (`.Rotation_5_ADDC5B57482A9A9A5491C3B6ED31BCB7` (break `/Game/Blueprints/Structs/TileInformation` _element)) 90.0))))
      (`PaperGroupedSpriteComponent.AddInstance` (`self.FourWayPaperGroupedSprite`) _returnvalue "/Game/Sprites/terrainFourWay_Sprite.terrainFourWay_Sprite" false (struct :`R` 1.0 :`G` 1.0 :`B` 1.0 :`A` 1.0))
      (`PaperGroupedSpriteComponent.AddInstance` (`self.BackgroundPaperGroupedSprite`) _returnvalue "/Game/Sprites/background_Sprite.background_Sprite" false (struct :`R` 1.0 :`G` 1.0 :`B` 1.0 :`A` 1.0) :!label _label)
      ;[1 1 1] keep track of how many we've created
      (`/Engine/EditorBlueprintResources/StandardMacros.IncrementInt` (`self.tilesCreated`)
        (:`  `
          _)))
    (:`Straight`
      (`PaperGroupedSpriteComponent.AddInstance` (`self.StraightPaperGroupedSprite`) _returnvalue "/Game/Sprites/terrainStraight_Sprite.terrainStraight_Sprite" false (struct :`R` 1.0 :`G` 1.0 :`B` 1.0 :`A` 1.0))
      (goto _label))
    (:`Three Way`
      (`PaperGroupedSpriteComponent.AddInstance` (`self.ThreeWayPaperGroupedSprite`) _returnvalue "/Game/Sprites/terrainThreeWay_Sprite.terrainThreeWay_Sprite" false (struct :`R` 1.0 :`G` 1.0 :`B` 1.0 :`A` 1.0))
      (goto _label))
    (:`Corner`
      (`PaperGroupedSpriteComponent.AddInstance` (`self.CornerPaperGroupedSprite`) _returnvalue "/Game/Sprites/terrainCorner_Sprite.terrainCorner_Sprite" false (struct :`R` 1.0 :`G` 1.0 :`B` 1.0 :`A` 1.0))
      (goto _label))
    (:`Dead End`
      (`PaperGroupedSpriteComponent.AddInstance` (`self.DeadEndPaperGroupedSprite`) _returnvalue "/Game/Sprites/terrainDeadEnd_Sprite.terrainDeadEnd_Sprite" false (struct :`R` 1.0 :`G` 1.0 :`B` 1.0 :`A` 1.0))
      (goto _label)))
  (return))

(fn `SetBottomVacancy`
  (params (xCheck :type Integer) (zCheck :type Integer))
  (returns (IsVacant :type Boolean))
  (locals (adjacentType :type Integer))
  (bind _returnvalue (or (`self.dontCheckDirections`) (== (`local.adjacentType`) -1)))
  ;[1 1 1] check if it's the first tile. If it is, then set the adjacent type variable to the vacant position(-1)
  (if (> (`self.tilesCreated`) 0)
    (bind _element (`self.GetTileInfo` xCheck (- zCheck 1)))
    (set `local.adjacentType` (break `/Game/Blueprints/Structs/TileInformation` _element))
    (else
      (set `local.adjacentType` -1)))
  (bind _element_2 (`self.GetTileInfo` xCheck zCheck))
  (`self.SetTileInfo` (make `/Game/Blueprints/Structs/TileInformation` (break `/Game/Blueprints/Structs/TileInformation` _element_2) (`.Rotation_5_ADDC5B57482A9A9A5491C3B6ED31BCB7` (break `/Game/Blueprints/Structs/TileInformation` _element_2)) (`.Openings_7_F7EF8F88495907CF6207A0B58024D475` (break `/Game/Blueprints/Structs/TileInformation` _element_2)) (`.Left_10_DB7199D24824B389FF47D582AEDECBFF` (break `/Game/Blueprints/Structs/TileInformation` _element_2)) (`.Right_14_58CFD1D541F441DB794B599FE93CD335` (break `/Game/Blueprints/Structs/TileInformation` _element_2)) (`.Top_15_FF8EB3A44EBFBDEC54CE4783EB41D170` (break `/Game/Blueprints/Structs/TileInformation` _element_2)) _returnvalue) xCheck zCheck)
  (return _returnvalue))

(fn `SetLeftVacancy`
  (params (xCheck :type Integer) (zCheck :type Integer))
  (returns (IsVacant :type Boolean))
  (locals (adjacentType :type Integer))
  (bind _returnvalue (or (`self.dontCheckDirections`) (== (`local.adjacentType`) -1)))
  (if (> (`self.tilesCreated`) 0)
    (bind _element (`self.GetTileInfo` (- xCheck 1) zCheck))
    (set `local.adjacentType` (break `/Game/Blueprints/Structs/TileInformation` _element))
    (else
      (set `local.adjacentType` -1)))
  (bind _element_2 (`self.GetTileInfo` xCheck zCheck))
  (`self.SetTileInfo` (make `/Game/Blueprints/Structs/TileInformation` (break `/Game/Blueprints/Structs/TileInformation` _element_2) (`.Rotation_5_ADDC5B57482A9A9A5491C3B6ED31BCB7` (break `/Game/Blueprints/Structs/TileInformation` _element_2)) (`.Openings_7_F7EF8F88495907CF6207A0B58024D475` (break `/Game/Blueprints/Structs/TileInformation` _element_2)) _returnvalue (`.Right_14_58CFD1D541F441DB794B599FE93CD335` (break `/Game/Blueprints/Structs/TileInformation` _element_2)) (`.Top_15_FF8EB3A44EBFBDEC54CE4783EB41D170` (break `/Game/Blueprints/Structs/TileInformation` _element_2)) (`.Down_16_1ABB1D3F4A6AF141A8692C870330AC01` (break `/Game/Blueprints/Structs/TileInformation` _element_2))) xCheck zCheck)
  (return _returnvalue))

(fn `SetRightVacancy`
  (params (xCheck :type Integer) (zCheck :type Integer))
  (returns (IsVacant :type Boolean))
  (locals (adjacentType :type Integer) (true :type Boolean :default true))
  (bind _returnvalue (or (`self.dontCheckDirections`) (== (`local.adjacentType`) -1)))
  (if (> (`self.tilesCreated`) 0)
    (bind _element (`self.GetTileInfo` (+ xCheck 1) zCheck))
    (set `local.adjacentType` (break `/Game/Blueprints/Structs/TileInformation` _element))
    (else
      (set `local.adjacentType` -1)))
  (bind _element_2 (`self.GetTileInfo` xCheck zCheck))
  (`self.SetTileInfo` (make `/Game/Blueprints/Structs/TileInformation` (break `/Game/Blueprints/Structs/TileInformation` _element_2) (`.Rotation_5_ADDC5B57482A9A9A5491C3B6ED31BCB7` (break `/Game/Blueprints/Structs/TileInformation` _element_2)) (`.Openings_7_F7EF8F88495907CF6207A0B58024D475` (break `/Game/Blueprints/Structs/TileInformation` _element_2)) (`.Left_10_DB7199D24824B389FF47D582AEDECBFF` (break `/Game/Blueprints/Structs/TileInformation` _element_2)) _returnvalue (`.Top_15_FF8EB3A44EBFBDEC54CE4783EB41D170` (break `/Game/Blueprints/Structs/TileInformation` _element_2)) (`.Down_16_1ABB1D3F4A6AF141A8692C870330AC01` (break `/Game/Blueprints/Structs/TileInformation` _element_2))) xCheck zCheck)
  (return _returnvalue))

(fn `SetTileInfo`
  (params (element :type "/Game/Blueprints/Structs/TileInformation Structure") (xSet :type Integer) (zSet :type Integer))
  ;[1 1 1] use this instead of insert, unless you want your array to grow
  (`KismetArrayLibrary.Array_Set` (`self.tileMap`) (+ xSet (* zSet (`self.width`))) element)
  (return))

(fn `SetTopVacancy`
  (params (xCheck :type Integer) (zCheck :type Integer))
  (returns (IsVacant :type Boolean))
  (locals (adjacentType :type Integer))
  (bind _returnvalue (or (`self.dontCheckDirections`) (== (`local.adjacentType`) -1)))
  (if (> (`self.tilesCreated`) 0)
    (bind _element (`self.GetTileInfo` xCheck (+ zCheck 1)))
    (set `local.adjacentType` (break `/Game/Blueprints/Structs/TileInformation` _element))
    (else
      (set `local.adjacentType` -1)))
  (bind _element_2 (`self.GetTileInfo` xCheck zCheck))
  (`self.SetTileInfo` (make `/Game/Blueprints/Structs/TileInformation` (break `/Game/Blueprints/Structs/TileInformation` _element_2) (`.Rotation_5_ADDC5B57482A9A9A5491C3B6ED31BCB7` (break `/Game/Blueprints/Structs/TileInformation` _element_2)) (`.Openings_7_F7EF8F88495907CF6207A0B58024D475` (break `/Game/Blueprints/Structs/TileInformation` _element_2)) (`.Left_10_DB7199D24824B389FF47D582AEDECBFF` (break `/Game/Blueprints/Structs/TileInformation` _element_2)) (`.Right_14_58CFD1D541F441DB794B599FE93CD335` (break `/Game/Blueprints/Structs/TileInformation` _element_2)) _returnvalue (`.Down_16_1ABB1D3F4A6AF141A8692C870330AC01` (break `/Game/Blueprints/Structs/TileInformation` _element_2))) xCheck zCheck)
  (return _returnvalue))

(fn `Shuffle`
  (params (numberOfInts :type Integer))
  (returns (randomInts :type "Array of Integer"))
  (locals (randomNumbers :type "Array of Integer") (firstRandomIndex :type Integer) (secondRandomIndex :type Integer) (storedValue :type Integer))
  (bind _returnvalue (- numberOfInts 1))
  (bind _randomnumbers (`local.randomNumbers`))
  (bind _randomnumbers_2 (`local.randomNumbers`))
  (bind _randomnumbers_3 (`local.randomNumbers`))
  (`KismetArrayLibrary.Array_Resize` _randomnumbers_2 numberOfInts)
  (for (_ _array_index) _randomnumbers_2
    ;[1 1 1] each element in our array is unique
    (`KismetArrayLibrary.Array_Set` _randomnumbers_2 _array_index _array_index))
  ;[1 1 1] shuffle 10 times
  (for _ (range 11)
    (bind _output_get (set `local.firstRandomIndex` (`KismetMathLibrary.RandomIntegerInRange` 0 _returnvalue)))
    (bind _output_get_2 (set `local.secondRandomIndex` (`KismetMathLibrary.RandomIntegerInRange` 0 _returnvalue)))
    ;[1 1 1] swap the values
    (set `local.storedValue` (`KismetArrayLibrary.Array_Get` _randomnumbers _output_get))
    (`KismetArrayLibrary.Array_Set` _randomnumbers_3 (`local.firstRandomIndex`) (`KismetArrayLibrary.Array_Get` _randomnumbers _output_get_2))
    (`KismetArrayLibrary.Array_Set` _randomnumbers_3 (`local.secondRandomIndex`) (`local.storedValue`)))
  (return _randomnumbers))

(fn `UserConstructionScript`
  (locals (loopCount :type Integer)))